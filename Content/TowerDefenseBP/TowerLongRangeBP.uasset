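; Long-range tower Blueprint for a tower defense game that automatically fires projectiles at enemy characters in range.
; FieldOfView overlap events add and remove EnemyCharacters in a range list, and Tick aims the Arrow component at the first entry.
; A ShouldShoot flag and a Delay scaled inversely by ShootSpeed throttle Shoot, which spawns a ProjectileBP from the Arrow with a slight pitch offset.
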(event OnComponentBeginOverlap(FieldOfView)
  (params (OverlappedComponent :type Primitive%20Component%20Object%20Reference) (OtherActor :type Actor%20Object%20Reference) (OtherComp :type Primitive%20Component%20Object%20Reference) (OtherBodyIndex :type Integer) (bFromSweep :type Boolean) (SweepResult :type Hit%20Result%20Structure%20%28by%20ref%29))
  (bind _asenemy_character (Utilities|Casting|CastToEnemyCharacter OtherActor))
  (Utilities|Array|AddUnique (Variables|Default|GetEnemiesOnRange) _asenemy_character))

(event OnComponentEndOverlap(FieldOfView)
  (params (OverlappedComponent :type Primitive%20Component%20Object%20Reference) (OtherActor :type Actor%20Object%20Reference) (OtherComp :type Primitive%20Component%20Object%20Reference) (OtherBodyIndex :type Integer))
  (bind _asenemy_character (Utilities|Casting|CastToEnemyCharacter OtherActor))
  (Utilities|Array|RemoveItem (Variables|Default|GetEnemiesOnRange) _asenemy_character))

(event EventTick
  (params (DeltaSeconds :type Float%20%28single-precision%29))
  (if (> (Utilities|Array|Length (Variables|Default|GetEnemiesOnRange)) 0)
    (Transformation|SetRelativeRotation (Variables|Default|GetArrow) (Math|Rotator|FindLookatRotation (Transformation|GetWorldLocation (Variables|Default|GetArrow)) (Transformation|GetActorLocation (Utilities|Array|Get(acopy) (Variables|Default|GetEnemiesOnRange)))) false false)
    (if (Variables|Default|GetShouldShoot)
      (Variables|Default|SetShouldShoot false)
      (CallFunction|Shoot)
      (Utilities|FlowControl|Delay (/ 1e+02 (Variables|Default|GetShootSpeed)))
      (Variables|Default|SetShouldShoot true))))

(fn ConstructionScript)

(fn Shoot
  (bind _arrow (Variables|Default|GetArrow))
  (bind _returnvalue (Transformation|GetWorldTransform _arrow))
  (bind (_roll _pitch _yaw) (Math|Rotator|BreakRotator (.rotation _returnvalue)))
  (Game|SpawnActorfromClass "/Game/TowerDefenseBP/ProjectileBP.ProjectileBP_C" (Math|Transform|MakeTransform (.location _returnvalue) (Math|Rotator|MakeRotator _roll (+ _pitch 5.0) _yaw) "1,1,1") "Undefined" 0 0)
  (Development|PrintString "SHOOT"))